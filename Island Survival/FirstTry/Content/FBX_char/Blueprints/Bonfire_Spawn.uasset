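; Bonfire build spot where the player spends firewood to construct a bonfire.
; A sphere overlap registers the spot on the Player as the current build location and clears it on exit.
; BuildBonfire checks and deducts firewood, spawns a Bonfire linked back to the spot, adds charcoal to the inventory, refreshes the HUD and disables the spot.
; ResetBuildSpot restores the marker mesh and collision for rebuilding.
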(event `self.Sphere.OnComponentBeginOverlap`
  (params (OverlappedComponent :type "PrimitiveComponent Object Reference") (OtherActor :type "Actor Object Reference") (OtherComp :type "PrimitiveComponent Object Reference") (OtherBodyIndex :type Integer) (bFromSweep :type Boolean) (SweepResult :type "HitResult Structure (by ref)"))
  (bind _asplayer (cast `/Game/FBX_char/Blueprints/Player` OtherActor))
  (set `/Game/FBX_char/Blueprints/Player.CurrentBonfireBuiltspot` self _asplayer))

(event `self.Sphere.OnComponentEndOverlap`
  (params (OverlappedComponent :type "PrimitiveComponent Object Reference") (OtherActor :type "Actor Object Reference") (OtherComp :type "PrimitiveComponent Object Reference") (OtherBodyIndex :type Integer))
  (bind _asplayer (cast `/Game/FBX_char/Blueprints/Player` OtherActor))
  (set `/Game/FBX_char/Blueprints/Player.CurrentBonfireBuiltspot` null _asplayer))

(fn `BuildBonfire`
  (params (PlayerRef :type "/Game/FBX_char/Blueprints/Player Object Reference"))
  (bind _firewoodcount (`/Game/FBX_char/Blueprints/Player.FirewoodCount` PlayerRef))
  (if (`self.BonfireBuilt`)
    _
    (elif (>= _firewoodcount (`self.RequiredFirewood`))
      (set `/Game/FBX_char/Blueprints/Player.FirewoodCount` (- _firewoodcount (`self.RequiredFirewood`)) PlayerRef)
      (bind _returnvalue (`|SpawnActorFromClass` "/Game/FBX_char/Blueprints/Bonfire.Bonfire_C" (`self.GetTransform`) "Undefined" "MultiplyWithRoot" null null))
      (`InventoryComponent.AddItem` (`/Game/FBX_char/Blueprints/Player.Inventory` PlayerRef) "Charcoal" 2)
      (set `/Game/FBX_char/Blueprints/Bonfire.BuildSpotRef` self _returnvalue)
      (set `self.BonfireBuilt` true)
      (`SceneComponent.SetVisibility` (`self.BuildSpotMesh`) false false)
      (`PrimitiveComponent.SetCollisionEnabled` (`self.Sphere`) "NoCollision")
      (bind _asplayer (cast `/Game/FBX_char/Blueprints/Player` (`GameplayStatics.GetPlayerCharacter` 0)))
      (`/Game/FBX_char/Blueprints/Player.RefreshHUD` _asplayer)
      (else
        (`KismetSystemLibrary.PrintString` "Not Enough Firewood")))))

(fn `resetBuildSpot`
  (set `self.BonfireBuilt` false)
  (`SceneComponent.SetVisibility` (`self.BuildSpotMesh`) true false)
  (`PrimitiveComponent.SetCollisionEnabled` (`self.Sphere`) "QueryOnly"))

(fn `UserConstructionScript`)