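; Coastline boundary actor that holds a CoastLine spline and can rebuild it as a circle around the actor's location.
; GenerateNewCircle, gated by the GenerateCircle flag, clears the spline and places NumPoints evenly spaced world-space points using Radius and ZHeight, then closes the loop.
; The event graph and construction script are empty, and nothing in this file calls the function.
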(fn `GenerateNewCircle`
  (bind _coastline (`self.CoastLine`))
  (bind _radius (`self.Radius`))
  (if (`self.GenerateCircle`)
    (`SplineComponent.ClearSplinePoints` (`self.CoastLine`) true)
    (for _index (range (`self.NumPoints`))
      (bind _returnvalue (* (`KismetMathLibrary.Conv_IntToDouble` _index) (/ 360.0 (`KismetMathLibrary.Conv_IntToDouble` (`self.NumPoints`)))))
      (`SplineComponent.AddSplinePoint` (`self.CoastLine`) (+ (`self.K2_GetActorLocation`) (`KismetMathLibrary.MakeVector` (* (`KismetMathLibrary.DegCos` _returnvalue) _radius) (* (`KismetMathLibrary.DegSin` _returnvalue) _radius) (`self.ZHeight`))) "World" true))
    (`SplineComponent.SetClosedLoop` _coastline true true)
    (`SplineComponent.UpdateSpline` _coastline)))

(fn `UserConstructionScript`)