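; GravelSpawner is an actor that scatters Gravel actors onto the surfaces around it when play begins.
; For each spawn count it picks random offsets within a square set by Radius at height Z, then line-traces downward on the Visibility channel.
; Each hit spawns a Gravel actor at the impact point with default rotation and scale, while misses spawn nothing.
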(event `self.ReceiveBeginPlay`
  (bind _radius (`self.Radius`))
  (bind _radius_2 (`self.Radius`))
  (bind _returnvalue (+ (`KismetMathLibrary.MakeVector` (`KismetMathLibrary.RandomFloatInRange` (`KismetMathLibrary.Conv_IntToDouble` (- 0 _radius)) (`KismetMathLibrary.Conv_IntToDouble` _radius)) (`KismetMathLibrary.RandomFloatInRange` (`KismetMathLibrary.Conv_IntToDouble` (- 0 _radius_2)) (`KismetMathLibrary.Conv_IntToDouble` _radius_2)) (`KismetMathLibrary.Conv_IntToDouble` (`self.Z`))) (`self.K2_GetActorLocation`)))
  (for _ (range (`self.spawncount`))
    (bind (_outhit _returnvalue_2) (`KismetSystemLibrary.LineTraceSingle` _returnvalue (- _returnvalue (0.0 0.0 5000.0)) "TraceTypeQuery1"))
    (if _returnvalue_2
      (`|SpawnActorFromClass` "/Game/FBX_char/Blueprints/Gravel.Gravel_C" (`KismetMathLibrary.MakeTransform` (`.ImpactPoint` (`GameplayStatics.BreakHitResult` _outhit))) "Undefined" "MultiplyWithRoot" null null))))

(fn `UserConstructionScript`)