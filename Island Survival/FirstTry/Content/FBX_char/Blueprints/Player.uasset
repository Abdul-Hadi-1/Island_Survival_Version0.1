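; Player character for a survival game, handling movement, sprinting, a swim-exit launch jump, HUD, pause and win/game-over screens.
; Interact acts on the first valid nearby reference: pickups, filter station, night-only sleep spot or fishing spot.
; Survival, inventory, cooking, fishing and water-filter components supply the logic, while lazily created puzzle widgets live in the HUD container.
; Eating, drinking, pickups and sleep refresh the HUD; reaching day 8 wins.
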(event `self.ReceiveBeginPlay`
  ;[0.005256 0.15 0.006761 0.5] HUD
  (bind _outactors (`GameplayStatics.GetAllActorsOfClass` "/Script/FirstTry.DayandNight"))
  (set `self.DayRef` (`|GetArrayItem` _outactors))
  (`|ExecutionSequence`
    (:`then_0`
      (bind _asplayer_controller (cast `PlayerController` (`self.GetController`)))
      (`EnhancedInputSubsystemInterface.AddMappingContext` (pcsubsystem `EnhancedInputLocalPlayerSubsystem` _asplayer_controller) "/Game/Inputs/InputA.InputA" 0 (struct)))
    (:`then_1`
      (bind _returnvalue (`|CreateWidget` "/Game/FBX_char/Blueprints/HUD.HUD_C" _asplayer_controller))
      (bind _output_get (set `self.Hudref` _returnvalue))
      (`UserWidget.AddToViewport` _output_get 0)
      (`self.RefreshHUD`)
      (`Widget.SetVisibility` (`/Game/FBX_char/Blueprints/HUD.HelpGuide` (`self.Hudref`)) "Visible")
      (set `self.HelpGuide` true)
      (bind _returnvalue_2 (`KismetSystemLibrary.K2_SetTimerDelegate` (`|CreateDelegate` :!event `HideHelpGuide`) 60.0))
      (set `self.AutoHideHelpGuide` _returnvalue_2)
      (add `SurvivalComp.OnPlayerDied` (`self.SurvivalComp`) (`|CreateDelegate` :!event `ShowGameOver`))
      (`KismetSystemLibrary.K2_SetTimerDelegate` (`|CreateDelegate` :!event `CheckWin`) 1.0 true))))

(event `EnhancedInput|/Game/Inputs/InputA_Move`
  (params (ActionValue :type "Vector2D Structure") (ElapsedSeconds :type "Float (double-precision)") (TriggeredSeconds :type "Float (double-precision)") (InputAction :type "InputAction Object Reference" :default "/Game/Inputs/InputA_Move.InputA_Move"))
  (bind (_x _y) (`KismetMathLibrary.BreakVector2D` ActionValue))
  ;[0 0.007163 0.15 0.5] Moving
  (:`Triggered`
    (`|ExecutionSequence`
      (:`then_0`
        (`self.AddMovementInput` (`self.GetActorForwardVector`) _y))
      (:`then_1`
        (`self.AddMovementInput` (`self.GetActorRightVector`) _x)))))

(event `self.K2_OnMovementModeChanged`
  (params (PrevMovementMode :type "EMovementMode Enum" :default "MOVE_None") (NewMovementMode :type "EMovementMode Enum" :default "MOVE_None") (PrevCustomMode :type Byte) (NewCustomMode :type Byte))
  ;[0.007269 0.15 0.02961 0.5] Setting Movement mode
  (set `self.Swimming` (or (`|EnumEquality` NewMovementMode "MOVE_Swimming") (`|EnumEquality` NewMovementMode "MOVE_Flying"))))

(event `RefreshHUD`
  (bind _inventory (`self.Inventory`))
  (bind _hudref (`self.Hudref`))
  (bind _dayref (`self.DayRef`))
  ;[0.005256 0.15 0.006761 0.5] HUD
  (`/Engine/EditorBlueprintResources/StandardMacros.IsValid` _hudref
    (:`Is Valid`
      (`/Engine/EditorBlueprintResources/StandardMacros.IsValid` _dayref
        (:`Is Valid`
          (`/Game/FBX_char/Blueprints/HUD.UpdateHUDValues` _hudref (`self.FirewoodCount`) (`InventoryComponent.GetItemCount` _inventory "UncookedFish") (`InventoryComponent.GetItemCount` _inventory "CookedFish") (`DayandNight.DayNumber` _dayref) (`InventoryComponent.GetItemCount` _inventory "Sand") (`InventoryComponent.GetItemCount` _inventory "Charcoal") (`InventoryComponent.GetItemCount` _inventory "Gravel") (`InventoryComponent.GetItemCount` _inventory "DirtyWater") (`InventoryComponent.GetItemCount` _inventory "CleanWater")))))))

(event `EnhancedInput|/Game/Inputs/InputA_Drinking`
  (params (ActionValue :type Boolean) (ElapsedSeconds :type "Float (double-precision)") (TriggeredSeconds :type "Float (double-precision)") (InputAction :type "InputAction Object Reference" :default "/Game/Inputs/InputA_Drinking.InputA_Drinking"))
  ;[0 0.018 0.15 0.5] Eating / Drinking
  (:`Started`
    (`SurvivalComp.Drinking` (`self.SurvivalComp`))
    (`self.RefreshHUD`)))

(event `EnhancedInput|/Game/Inputs/InputA_Look`
  (params (ActionValue :type "Vector2D Structure") (ElapsedSeconds :type "Float (double-precision)") (TriggeredSeconds :type "Float (double-precision)") (InputAction :type "InputAction Object Reference" :default "/Game/Inputs/InputA_Look.InputA_Look"))
  (bind (_x _y) (`KismetMathLibrary.BreakVector2D` ActionValue))
  ;[0 0.01839 0.15 0.5] Looking
  (:`Triggered`
    (`|ExecutionSequence`
      (:`then_0`
        (`self.AddControllerYawInput` _x))
      (:`then_1`
        (`self.AddControllerPitchInput` _y)))))

(event `ShowGameOver`
  ;[0.005256 0.15 0.006761 0.5] HUD
  (`Widget.SetVisibility` (`/Game/FBX_char/Blueprints/HUD.GameOverOverlay` (`self.Hudref`)) "Visible")
  (bind _asplayer_controller (cast `PlayerController` (`self.GetController`)))
  (set `PlayerController.bShowMouseCursor` true _asplayer_controller)
  (`WidgetBlueprintLibrary.SetInputMode_UIOnlyEx` _asplayer_controller null)
  (`CharacterMovementComponent.DisableMovement` (`self.CharacterMovement`)))

(event `EnhancedInput|/Game/Inputs/InputA_Sprint`
  (params (ActionValue :type Boolean) (ElapsedSeconds :type "Float (double-precision)") (TriggeredSeconds :type "Float (double-precision)") (InputAction :type "InputAction Object Reference" :default "/Game/Inputs/InputA_Sprint.InputA_Sprint"))
  (bind _charactermovement (`self.CharacterMovement`))
  ;[0 0.04444 0.15 0.5] Sprinting
  (:`Triggered`
    (set `CharacterMovementComponent.MaxWalkSpeed` 1000.0 _charactermovement))
  (:`Canceled`
    (set `CharacterMovementComponent.MaxWalkSpeed` 500.0 _charactermovement :!label _label))
  (:`Completed`
    (goto _label)))

(event `EnhancedInput|/Game/Inputs/InputA_Jump`
  (params (ActionValue :type Boolean) (ElapsedSeconds :type "Float (double-precision)") (TriggeredSeconds :type "Float (double-precision)") (InputAction :type "InputAction Object Reference" :default "/Game/Inputs/InputA_Jump.InputA_Jump"))
  (bind _charactermovement (`self.CharacterMovement`))
  ;[0 0.01758 0.15 0.5] Jumping
  (:`Started`
    (if (`self.Swimming`)
      (`ActorComponent.SetComponentTickEnabled` (`self.Swim`) false)
      (`MovementComponent.StopMovementImmediately` _charactermovement)
      (`CharacterMovementComponent.SetMovementMode` _charactermovement "MOVE_Falling" 0)
      (`self.LaunchCharacter` (+ (* (`self.GetActorForwardVector`) 1500.0) (`KismetMathLibrary.MakeVector` 0.0 0.0 4200.0)) true true)
      (`KismetSystemLibrary.Delay` 0.9)
      (`ActorComponent.SetComponentTickEnabled` (`self.Swim`) true)
      (else
        (`self.Jump`)))))

(event `CheckWin`
  ;[0.005256 0.15 0.006761 0.5] HUD
  (if (not (`self.HasWon`))
    (if (>= (`DayandNight.DayNumber` (`self.DayRef`)) 8)
      (set `self.HasWon` true)
      (`self.ShowYouWon`))))

(event `EnhancedInput|/Game/Inputs/InputA_Eating`
  (params (ActionValue :type Boolean) (ElapsedSeconds :type "Float (double-precision)") (TriggeredSeconds :type "Float (double-precision)") (InputAction :type "InputAction Object Reference" :default "/Game/Inputs/InputA_Eating.InputA_Eating"))
  ;[0 0.018 0.15 0.5] Eating / Drinking
  (:`Started`
    (`SurvivalComp.Eating` (`self.SurvivalComp`))
    (`self.RefreshHUD`)))

(event `ShowYouWon`
  ;[0.005256 0.15 0.006761 0.5] HUD
  (`Widget.SetVisibility` (`/Game/FBX_char/Blueprints/HUD.YouSurvivedOverlay` (`self.Hudref`)) "Visible")
  (bind _asplayer_controller (cast `PlayerController` (`self.GetController`)))
  (set `PlayerController.bShowMouseCursor` true _asplayer_controller)
  (`WidgetBlueprintLibrary.SetInputMode_UIOnlyEx` _asplayer_controller null)
  (`CharacterMovementComponent.DisableMovement` (`self.CharacterMovement`)))

(event `ShowPauseMenu`
  ;[0.005256 0.15 0.006761 0.5] HUD
  (`GameplayStatics.SetGamePaused` true)
  (set `Widget.Visibility` "Visible" (`/Game/FBX_char/Blueprints/HUD.PauseMenuOverlay` (`self.Hudref`)))
  (bind _asplayer_controller (cast `PlayerController` (`self.GetController`)))
  (bind _output_get (set `PlayerController.bShowMouseCursor` true _asplayer_controller))
  (`WidgetBlueprintLibrary.SetInputMode_GameAndUIEx` _asplayer_controller null "DoNotLock" _output_get))

(event `EnhancedInput|/Game/Inputs/InputA_HelpGuide`
  (params (ActionValue :type Boolean) (ElapsedSeconds :type "Float (double-precision)") (TriggeredSeconds :type "Float (double-precision)") (InputAction :type "InputAction Object Reference" :default "/Game/Inputs/InputA_HelpGuide.InputA_HelpGuide"))
  ;[0.005256 0.15 0.006761 0.5] HelpGuide Show/Hide
  (:`Started`
    (if (`self.HelpGuide`)
      (`Widget.SetVisibility` (`/Game/FBX_char/Blueprints/HUD.HelpGuide` (`self.Hudref`)) "Hidden")
      (set `self.HelpGuide` false)
      (`KismetSystemLibrary.K2_ClearAndInvalidateTimerHandle` (`self.AutoHideHelpGuide`))
      (else
        (`Widget.SetVisibility` (`/Game/FBX_char/Blueprints/HUD.HelpGuide` (`self.Hudref`)) "Visible")
        (set `self.HelpGuide` true)))))

(event `HIdePauseMenu`
  ;[0.005256 0.15 0.006761 0.5] HUD
  (`GameplayStatics.SetGamePaused` false)
  (set `Widget.Visibility` "Collapsed" (`/Game/FBX_char/Blueprints/HUD.PauseMenuOverlay` (`self.Hudref`)))
  (bind _asplayer_controller (cast `PlayerController` (`self.GetController`)))
  (set `PlayerController.bShowMouseCursor` false _asplayer_controller)
  (`WidgetBlueprintLibrary.SetInputMode_GameOnly` _asplayer_controller))

(event `EnhancedInput|/Game/Inputs/InputA_Pause`
  (params (ActionValue :type Boolean) (ElapsedSeconds :type "Float (double-precision)") (TriggeredSeconds :type "Float (double-precision)") (InputAction :type "InputAction Object Reference" :default "/Game/Inputs/InputA_Pause.InputA_Pause"))
  ;[0.005256 0.15 0.006761 0.5] HUD
  (:`Started`
    (if (`GameplayStatics.IsGamePaused`)
      (`self.HIdePauseMenu`)
      (else
        (`self.ShowPauseMenu`)))))

(event `HideHelpGuide`
  ;[0.005256 0.15 0.006761 0.5] HelpGuide Show/Hide
  (`Widget.SetVisibility` (`/Game/FBX_char/Blueprints/HUD.HelpGuide` (`self.Hudref`)) "Hidden")
  (set `self.HelpGuide` false))

(event `Hide Water Puzzle`
  (bind _waterfilterpuzzleref (`self.WaterFilterPuzzleRef`))
  ;[0.15 0.1022 0 0.502] Show/Hide Purifing Puzzle
  (`/Engine/EditorBlueprintResources/StandardMacros.IsValid` _waterfilterpuzzleref
    (:`Is Valid`
      (`KismetSystemLibrary.Delay` 0.2)
      (`Widget.SetVisibility` _waterfilterpuzzleref "Hidden")
      (`self.RefreshHUD`))))

(event `ShowCookingPuzzle_Event`
  (bind _cooking (`self.Cooking`))
  (bind _cookingpuzzleref (`self.Cookingpuzzleref`))
  (bind _cooking_2 (`self.Cooking`))
  ;[0.15 0.1022 0 0.502] Show/Hide Cooking Puzzle
  (`KismetSystemLibrary.Delay` 0.8)
  (`/Engine/EditorBlueprintResources/StandardMacros.IsValid` _cookingpuzzleref
    (:`Is Valid`
      (`/Game/FBX_char/Blueprints/JigsawPuzzle_Cooking.InitPuzzle` (`self.Cookingpuzzleref`) (`CookingComponent.GetCookingPuzzleGridSize` _cooking) (`CookingComponent.GetCookingPuzzleTimeLimit` _cooking))
      (cast `PlayerController` (`self.GetController`))
      (`Widget.SetVisibility` _cookingpuzzleref "Visible"))
    (:`Is Not Valid`
      (bind _asplayer_controller (cast `PlayerController` (`self.GetController`)))
      (bind _returnvalue (`|CreateWidget` "/Game/FBX_char/Blueprints/JigsawPuzzle_Cooking.JigsawPuzzle_Cooking_C" _asplayer_controller))
      (bind _output_get (set `self.Cookingpuzzleref` _returnvalue))
      (`Overlay.AddChildToOverlay` (`/Game/FBX_char/Blueprints/HUD.PuzzleContainer` (`self.Hudref`)) _output_get)
      (`/Game/FBX_char/Blueprints/JigsawPuzzle_Cooking.InitPuzzle` (`self.Cookingpuzzleref`) (`CookingComponent.GetCookingPuzzleGridSize` _cooking_2) (`CookingComponent.GetCookingPuzzleTimeLimit` _cooking_2)))))

(event `ShowFishingPuzzle_Event`
  (bind _puzzleref (`self.PuzzleRef`))
  (bind _fishingpuzzlemanager (`self.FishingPuzzleManager`))
  (bind _fishingpuzzlemanager_2 (`self.FishingPuzzleManager`))
  ;[0.15 0.1022 0 0.502] Show/Hide Fishing Puzzle
  (`KismetSystemLibrary.Delay` 0.8)
  (`/Engine/EditorBlueprintResources/StandardMacros.IsValid` _puzzleref
    (:`Is Valid`
      (`/Game/FBX_char/Blueprints/JigsawPuzzle.InitPuzzle` (`self.PuzzleRef`) (`FishingPuzzleManager.GetFishingPuzzleGridSize` _fishingpuzzlemanager) (`FishingPuzzleManager.GetFishingPuzzleTimeLimit` _fishingpuzzlemanager))
      (bind _asplayer_controller (cast `PlayerController` (`self.GetController`)))
      (`Widget.SetVisibility` _puzzleref "Visible")
      (set `PlayerController.bShowMouseCursor` true _asplayer_controller)
      (`WidgetBlueprintLibrary.SetInputMode_GameAndUIEx` _asplayer_controller (`self.PuzzleRef`) "DoNotLock" false))
    (:`Is Not Valid`
      (bind _asplayer_controller_2 (cast `PlayerController` (`self.GetController`)))
      (bind _returnvalue (`|CreateWidget` "/Game/FBX_char/Blueprints/JigsawPuzzle.JigsawPuzzle_C" _asplayer_controller_2))
      (bind _output_get (set `self.PuzzleRef` _returnvalue))
      (`Overlay.AddChildToOverlay` (`/Game/FBX_char/Blueprints/HUD.PuzzleContainer` (`self.Hudref`)) _output_get)
      (`/Game/FBX_char/Blueprints/JigsawPuzzle.InitPuzzle` (`self.PuzzleRef`) (`FishingPuzzleManager.GetFishingPuzzleGridSize` _fishingpuzzlemanager_2) (`FishingPuzzleManager.GetFishingPuzzleTimeLimit` _fishingpuzzlemanager_2))
      (set `PlayerController.bShowMouseCursor` true _asplayer_controller_2)
      (`WidgetBlueprintLibrary.SetInputMode_GameAndUIEx` _asplayer_controller_2 (`self.PuzzleRef`) "DoNotLock" false))))

(event `Show Water Puzzle`
  (bind _waterfilterpuzzleref (`self.WaterFilterPuzzleRef`))
  ;[0.15 0.1022 0 0.502] Show/Hide Purifing Puzzle
  (`/Engine/EditorBlueprintResources/StandardMacros.IsValid` _waterfilterpuzzleref
    (:`Is Valid`
      (`Widget.SetVisibility` _waterfilterpuzzleref "Visible"))
    (:`Is Not Valid`
      (bind _returnvalue (`|CreateWidget` "/Game/FBX_char/Blueprints/WaterFilterPuzzle.WaterFilterPuzzle_C" (`GameplayStatics.GetPlayerController` 0)))
      (bind _output_get (set `self.WaterFilterPuzzleRef` _returnvalue))
      (`Overlay.AddChildToOverlay` (`/Game/FBX_char/Blueprints/HUD.PuzzleContainer` (`self.Hudref`)) _returnvalue)
      (`Widget.SetVisibility` _output_get "Visible"))))

(event `HideCookingPuzzle_Event`
  ;[0.15 0.1022 0 0.502] Show/Hide Cooking Puzzle
  (`KismetSystemLibrary.Delay` 0.2)
  (`Widget.SetVisibility` (`self.Cookingpuzzleref`) "Hidden")
  (`self.RefreshHUD`))

(event `HideFishingPuzzle_Event`
  ;[0.15 0.1022 0 0.502] Show/Hide Fishing Puzzle
  (`KismetSystemLibrary.Delay` 0.0)
  (bind _asplayer_controller (cast `PlayerController` (`self.GetController`)))
  (`Widget.SetVisibility` (`self.PuzzleRef`) "Hidden")
  (set `PlayerController.bShowMouseCursor` false _asplayer_controller)
  (`WidgetBlueprintLibrary.SetInputMode_GameOnly` _asplayer_controller)
  (`/Game/FBX_char/Assets-For-Use/FishingRod_Blueprint.StopFishing` (`self.CurrentFishingSpot`) self))

(event `EnhancedInput|/Game/Inputs/InputB_Bonfire`
  (params (ActionValue :type Boolean) (ElapsedSeconds :type "Float (double-precision)") (TriggeredSeconds :type "Float (double-precision)") (InputAction :type "InputAction Object Reference" :default "/Game/Inputs/InputB_Bonfire.InputB_Bonfire"))
  ;[0.15 0.1022 0 0.502] Bonfire
  (:`Started`
    (`/Engine/EditorBlueprintResources/StandardMacros.IsValid` (`self.CurrentBonfireBuiltspot`)
      (:`Is Valid`
        (`KismetSystemLibrary.PrintString` "Player in Campfire area")
        (`/Game/FBX_char/Blueprints/Bonfire_Spawn.BuildBonfire` (`self.CurrentBonfireBuiltspot`) self))
      (:`Is Not Valid`
        (`KismetSystemLibrary.PrintString` "Player not in Campfire area")))))

(event `EnhancedInput|/Game/Inputs/InputA_Interact`
  (params (ActionValue :type Boolean) (ElapsedSeconds :type "Float (double-precision)") (TriggeredSeconds :type "Float (double-precision)") (InputAction :type "InputAction Object Reference" :default "/Game/Inputs/InputA_Interact.InputA_Interact"))
  (bind _currentfirewood (`self.CurrentFirewood`))
  (bind _currentsand (`self.CurrentSand`))
  (bind _currentgravel (`self.CurrentGravel`))
  (bind _currentwater (`self.CurrentWater`))
  (bind _dayref (`self.DayRef`))
  ;[0.15 0.1022 0 0.502] Interaction
  (:`Started`
    (`/Engine/EditorBlueprintResources/StandardMacros.IsValid` _currentfirewood
      (:`Is Valid`
        (`/Game/FBX_char/Blueprints/Firewood.pickupfirewood` _currentfirewood self)
        (set `self.CurrentFirewood` null)
        (`self.RefreshHUD`))
      (:`Is Not Valid`
        (`/Engine/EditorBlueprintResources/StandardMacros.IsValid` _currentsand
          (:`Is Valid`
            (`/Game/FBX_char/Blueprints/Sand.pickupSand` _currentsand self)
            (set `self.CurrentSand` null)
            (`self.RefreshHUD`))
          (:`Is Not Valid`
            (`/Engine/EditorBlueprintResources/StandardMacros.IsValid` _currentgravel
              (:`Is Valid`
                (`/Game/FBX_char/Blueprints/Gravel.pickupGravel` _currentgravel self)
                (set `self.CurrentGravel` null)
                (`self.RefreshHUD`))
              (:`Is Not Valid`
                (`/Engine/EditorBlueprintResources/StandardMacros.IsValid` _currentwater
                  (:`Is Valid`
                    (`/Game/FBX_char/Blueprints/WaterCollector.PickUpDirtyWater` _currentwater self)
                    (set `self.CurrentWater` null)
                    (`self.RefreshHUD`))
                  (:`Is Not Valid`
                    (`/Engine/EditorBlueprintResources/StandardMacros.IsValid` (`self.CurrentFilterStation`)
                      (:`Is Valid`
                        (if (`WaterFilter.CanStartPurifying` (`self.WaterFilter`))
                          (`self.Show Water Puzzle`)
                          (`WaterFilter.StartPurifying` (`self.WaterFilter`) (`self.WaterFilterPuzzleRef`))
                          (else
                            (`KismetSystemLibrary.PrintString` "Missing Materials"))))
                      (:`Is Not Valid`
                        (`/Engine/EditorBlueprintResources/StandardMacros.IsValid` (`self.CurrentSleepSpot`)
                          (:`Is Valid`
                            (if (`DayandNight.IsNightTime` _dayref)
                              (`SurvivalComp.AdvanceSurvivalByHours` (`self.SurvivalComp`) (`DayandNight.GetHoursUntilMorning` _dayref 0.25))
                              (`DayandNight.SkipToMorning` _dayref 0.25)
                              (`self.RefreshHUD`)
                              (else
                                (`KismetSystemLibrary.PrintString` "You can only Sleep at Night"))))
                          (:`Is Not Valid`
                            ;; Fishing
                            (if (`self.inInteraction`)
                              (`/Engine/EditorBlueprintResources/StandardMacros.IsValid` (`self.CurrentFishingSpot`)
                                (:`Is Valid`
                                  (`/Game/FBX_char/Assets-For-Use/FishingRod_Blueprint.StopFishing` (`self.CurrentFishingSpot`) self)
                                  (set `self.inInteraction` false)
                                  (set `self.CurrentFishingSpot` null)))
                              (else
                                (`/Engine/EditorBlueprintResources/StandardMacros.IsValid` (`self.CurrentFishingSpot`)
                                  (:`Is Valid`
                                    (`/Game/FBX_char/Assets-For-Use/FishingRod_Blueprint.StartFishing` (`self.CurrentFishingSpot`) self)
                                    (set `self.inInteraction` true)))))))))))))))))))

(event `EnhancedInput|/Game/Inputs/InputC_Cooking`
  (params (ActionValue :type Boolean) (ElapsedSeconds :type "Float (double-precision)") (TriggeredSeconds :type "Float (double-precision)") (InputAction :type "InputAction Object Reference" :default "/Game/Inputs/InputC_Cooking.InputC_Cooking"))
  ;[0.15 0.1022 0 0.502] Cooking
  (:`Started`
    (`/Engine/EditorBlueprintResources/StandardMacros.IsValid` (`self.CurrentBonfire`)
      (:`Is Valid`
        (if (`CookingComponent.CanStartCooking` (`self.Cooking`))
          (`self.ShowCookingPuzzle_Event`)
          (`CookingComponent.StartCooking` (`self.Cooking`) (`self.Cookingpuzzleref`))
          (else
            (`KismetSystemLibrary.PrintString` "No Uncooked Fish"))))
      (:`Is Not Valid`
        (`KismetSystemLibrary.PrintString` "Cooking Not Started")))))

(fn `UserConstructionScript`)