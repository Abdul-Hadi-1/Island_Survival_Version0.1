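; Bonfire actor, apparently player-built, that serves as a cooking point and lasts until the in-game day changes.
; It records the DayandNight day number at BeginPlay and polls it on Tick.
; When a later day arrives it adds Charcoal to the player's inventory wherever they are, resets its build spot and destroys itself.
; CookingSphere overlaps set and clear the player's CurrentBonfire reference.
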(event `self.ReceiveBeginPlay`
  (bind _returnvalue (`GameplayStatics.GetActorOfClass` "/Script/FirstTry.DayandNight"))
  (bind _output_get (set `self.DayandNightRef` _returnvalue))
  (set `self.SpawnDay` (`DayandNight.DayNumber` _output_get)))

(event `self.ReceiveTick`
  (params (DeltaSeconds :type "Float (single-precision)"))
  (bind _dayandnightref (`self.DayandNightRef`))
  (bind _buildspotref (`self.BuildSpotRef`))
  (if (not (`self.FireExpired`))
    (`/Engine/EditorBlueprintResources/StandardMacros.IsValid` _dayandnightref
      (:`Is Valid`
        (if (> (`DayandNight.DayNumber` _dayandnightref) (`self.SpawnDay`))
          (set `self.FireExpired` true)
          (bind _asplayer (cast `/Game/FBX_char/Blueprints/Player` (`GameplayStatics.GetPlayerPawn` 0)))
          (`InventoryComponent.AddItem` (`/Game/FBX_char/Blueprints/Player.Inventory` _asplayer) "Charcoal" 2)
          (`/Game/FBX_char/Blueprints/Player.RefreshHUD` _asplayer)
          (`/Engine/EditorBlueprintResources/StandardMacros.IsValid` _buildspotref
            (:`Is Valid`
              (`/Game/FBX_char/Blueprints/Bonfire_Spawn.resetBuildSpot` _buildspotref))
            (:`Is Not Valid`
              _))
          (`self.K2_DestroyActor`))))))

(event `self.CookingSphere.OnComponentBeginOverlap`
  (params (OverlappedComponent :type "PrimitiveComponent Object Reference") (OtherActor :type "Actor Object Reference") (OtherComp :type "PrimitiveComponent Object Reference") (OtherBodyIndex :type Integer) (bFromSweep :type Boolean) (SweepResult :type "HitResult Structure (by ref)"))
  (bind _asplayer (cast `/Game/FBX_char/Blueprints/Player` OtherActor))
  (set `/Game/FBX_char/Blueprints/Player.CurrentBonfire` self _asplayer))

(event `self.CookingSphere.OnComponentEndOverlap`
  (params (OverlappedComponent :type "PrimitiveComponent Object Reference") (OtherActor :type "Actor Object Reference") (OtherComp :type "PrimitiveComponent Object Reference") (OtherBodyIndex :type Integer))
  (bind _asplayer (cast `/Game/FBX_char/Blueprints/Player` OtherActor))
  (set `/Game/FBX_char/Blueprints/Player.CurrentBonfire` null _asplayer))

(fn `UserConstructionScript`)