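; Ocean blocker actor that lines a coastline spline with wall segments, apparently to act as a boundary at the water's edge.
; Its construction script takes the spline from CoastlineBoundry, clears the wall HISM and adds a world-space instance at each segment-length step.
; Each instance follows the spline's rotation, with a height offset and scale from segment length, thickness and height.
; The script prints the instance count; the event graph is empty.
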(event `self.ReceiveBeginPlay`)

(fn `UserConstructionScript`
  (`InstancedStaticMeshComponent.ClearInstances` (`self.WallHISM`))
  (bind _output_get (set `self.OceanSpline` (`/Game/FBX_char/Blueprints/Coastline_Boundry.CoastLine` (`self.Coastline Boundry`))))
  (for _index (range (+ (`KismetMathLibrary.FFloor` (/ (`SplineComponent.GetSplineLength` _output_get) (`self.SegmentLength`))) 1))
    (bind _output_get_2 (set `self.Distance` (* (`KismetMathLibrary.Conv_IntToDouble` _index) (`self.SegmentLength`))))
    (`InstancedStaticMeshComponent.AddInstance` (`self.WallHISM`) (`KismetMathLibrary.MakeTransform` (`KismetMathLibrary.MakeVector` (.x (.location (`SplineComponent.GetTransformAtDistanceAlongSpline` (`self.OceanSpline`) _output_get_2 "World" false))) (.y (.location (`SplineComponent.GetTransformAtDistanceAlongSpline` (`self.OceanSpline`) _output_get_2 "World" false))) (+ (.z (.location (`SplineComponent.GetTransformAtDistanceAlongSpline` (`self.OceanSpline`) _output_get_2 "World" false))) (`self.ZOffset`))) (.rotation (`SplineComponent.GetTransformAtDistanceAlongSpline` (`self.OceanSpline`) _output_get_2 "World" false)) (`KismetMathLibrary.MakeVector` (/ (`self.SegmentLength`) 100.0) (/ (`self.WallThickness`) 100.0) (/ (`self.WallHeight`) 100.0))) true))
  (`KismetSystemLibrary.PrintString` (`KismetStringLibrary.Conv_IntToString` (`InstancedStaticMeshComponent.GetInstanceCount` (`self.WallHISM`))) true true (struct :`G` 0.66 :`B` 1.0 :`A` 1.0) 100.0))